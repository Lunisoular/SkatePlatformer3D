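; BP_Gate is a gate Blueprint that opens once when its OpenGate event is called.
; A DoOnce guard starts the LS_GateOpens level sequence, then after a short delay plays a 2D opening sound and a timeline.
; The timeline moves the SMFence010 component along relative Z, scaling its location track by OpenLocation.
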(event Custom|OpenGate
  (Utilities|FlowControl|DoOnce false
    (:Completed
      (bind _outactor (Sequencer|Player|CreateLevelSequencePlayer "/Game/BP/Cinematics/LS_GateOpens.LS_GateOpens"))
      (Sequencer|Player|Play (Variables|/Script/LevelSequence.LevelSequenceActor|GetSequencePlayer _outactor) :!class /Script/MovieScene.MovieSceneSequencePlayer)
      (Utilities|FlowControl|Delay 0.1)
      (Audio|PlaySound2D "/Game/Sounds/Other_SFX/GateOpeningSFX.GateOpeningSFX" 0.8 1.0 0.0 0 0)
      (bind _location (Timeline|Timeline Play)
        (:Update
          (Transformation|SetRelativeLocation (Variables|Default|GetSM_Fence_010) (Math|Vector|MakeVector 0.0 0.0 (* _location (Variables|Default|GetOpenLocation))) false false))))))

(fn ConstructionScript)