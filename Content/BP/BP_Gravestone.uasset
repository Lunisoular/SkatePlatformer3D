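; BP_Gravestone is a gravestone prop that varies its static mesh's appearance at BeginPlay, leaving the construction script empty.
; It randomizes height offset and tilt, then picks a cone or cylinder mesh, with cone listed twice.
; The random yaw is overwritten by the following tilt rotation, which zeroes it.
; Scale resolves to MaxSize on every axis because both random bounds are equal.
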(event EventBeginPlay
  (bind _maxheightoffset (Variables|Default|GetMaxHeightOffset))
  (bind _maxrotationangle (Variables|Default|GetMaxRotationAngle))
  (bind _maxpitchrollangle (Variables|Default|GetMaxPitchRollAngle))
  (bind _maxsize (Variables|Default|GetMaxSize))
  (bind _returnvalue (* _maxpitchrollangle -1.0))
  (bind _returnvalue_2 (* _maxsize 1.0))
  (bind _returnvalue_3 (Math|Random|RandomFloatinRange _returnvalue _maxpitchrollangle))
  (bind _returnvalue_4 (Math|Random|RandomFloatinRange _returnvalue_2 _maxsize))
  ;[0.15 0.15 0.15 0.5] Zufälliger Offset (Z-Achse)
  (Transformation|AddWorldOffset (Variables|Default|GetMesh) (Math|Vector|MakeVector 0.0 0.0 (Math|Random|RandomFloatinRange (* _maxheightoffset -1.0) _maxheightoffset)) false false)
  ;[0.15 0.15 0.15 0.5] Zufällige Rotation (Z-Achse)
  (Transformation|SetWorldRotation (Variables|Default|GetMesh) (Math|Rotator|MakeRotator 0.0 0.0 (Math|Random|RandomFloatinRange (* _maxrotationangle -1.0) _maxrotationangle)) false false)
  ;[0.15 0.15 0.15 0.5] Zufällige Neigung (20 Grad, X- und Y-Achse)
  (Transformation|SetWorldRotation (Variables|Default|GetMesh) (Math|Rotator|MakeRotator _returnvalue_3 _returnvalue_3 0.0) false false)
  ;[0.15 0.15 0.15 0.5] Zufällige Größe (20% größer oder kleiner)
  (Transformation|SetWorldScale3D (Variables|Default|GetMesh) (Math|Vector|MakeVector _returnvalue_4 _returnvalue_4 _returnvalue_4))
  ;[0.15 0.15 0.15 0.5] Zufälliges Mesh (3 mögliche Variationen)
  (Components|StaticMesh|SetStaticMesh (Variables|Default|GetMesh) (.OutItem (Utilities|Array|Random (Utilities|Array|MakeArray "/Engine/BasicShapes/Cone.Cone" "/Engine/BasicShapes/Cylinder.Cylinder" "/Engine/BasicShapes/Cone.Cone")))))

(fn ConstructionScript)