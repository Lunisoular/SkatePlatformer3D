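; BP_Collectible is a soul pickup that BP_Grimmy collects by touching it.
; Tick keeps calling Play on a Timeline, whose Loc and Rot tracks drive the mesh's relative height and yaw for an animated bob and spin.
; On sphere overlap with BP_Grimmy, it adds a soul through the BP_HUD collectibles widget, plays a confirm sound, disables the sphere's collision and destroys itself.
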(event OnComponentBeginOverlap(Sphere)
  (params (OverlappedComponent :type Primitive%20Component%20Object%20Reference) (OtherActor :type Actor%20Object%20Reference) (OtherComp :type Primitive%20Component%20Object%20Reference) (OtherBodyIndex :type Integer) (bFromSweep :type Boolean) (SweepResult :type Hit%20Result%20Structure%20%28by%20ref%29))
  (Utilities|Casting|CastToBP_Grimmy OtherActor)
  (bind _asbp_hud (Utilities|Casting|CastToBP_HUD (HUD|GetHUD (Game|GetPlayerController 0))))
  (Default|CollectSouls (Variables|/Game/UI/BP_HUD.BP_HUD_C|GetCollectiblesWidget _asbp_hud) 1)
  (Audio|PlaySound2D "/Game/Sounds/UI_SFX/ButtonSFXConfirm.ButtonSFXConfirm" 1.0 1.0 0.0 0 0)
  (Collision|SetCollisionEnabled (Variables|Default|GetSphere) "NoCollision")
  (Actor|DestroyActor))

(event EventTick
  (params (DeltaSeconds :type Float%20%28single-precision%29))
  (bind _mesh (Variables|Default|GetMesh))
  (bind _relativerotation (Variables|/Script/Engine.SceneComponent|GetRelativeRotation _mesh))
  (bind (_direction _loc _rot) (Timeline|Timeline Play)
    (:Update
      (Transformation|SetRelativeLocationAndRotation (Variables|Default|GetMesh) (Math|Vector|MakeVector 0.0 0.0 (* _loc 4e+01)) (Math|Rotator|MakeRotator (.roll _relativerotation) (.pitch _relativerotation) (* _rot 3.6e+02)) false false))))

(fn ConstructionScript)