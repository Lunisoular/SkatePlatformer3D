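; BP_Enemy is a hazard enemy that starts chasing the player once they come within its sensor radius.
; Tick compares the distance to the player pawn against the scaled radius of the SensorRadius sphere, rather than using overlap events.
; A DoOnce triggers the chase a single time.
; AI MoveTo then re-issues itself one tick after every success or failure, so the pursuit continues regardless of range.
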(event Custom|StartChasingPlayer
  (AI|AIMoveTo self "0, 0, 0" (Game|Player|GetPlayerPawn 0) 2e+01 false
    (:OnSuccess
      _)
    (:OnFail
      _))
  (Utilities|FlowControl|DelayUntilNextTick)
  (CallFunction|StartChasingPlayer))

(event EventTick
  (params (DeltaSeconds :type Float%20%28single-precision%29))
  (if (CallFunction|IsSensingPlayer)
    (Utilities|FlowControl|DoOnce false
      (:Completed
        (CallFunction|StartChasingPlayer)))))

(fn ConstructionScript)

(fn IsSensingPlayer
  (return (< (Math|Vector|VectorLength (- (Transformation|GetActorLocation (Game|Player|GetPlayerPawn 0)) (Transformation|GetActorLocation))) (Components|Sphere|GetScaledSphereRadius (Variables|Default|GetSensorRadius)))))