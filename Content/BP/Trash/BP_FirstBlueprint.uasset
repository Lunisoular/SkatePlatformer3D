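; BP_FirstBlueprint is an actor, apparently a first Blueprint exercise, with a mesh and a point light that drifts steadily upward.
; BeginPlay raises, rotates and scales the mesh, then swaps it to a pyramid.
; Tick moves the root up, scaled by delta time, and uses a Delay to randomize light intensity and pick one of four colors about once a second.
; Overlap and hit events are empty.
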(event EventBeginPlay
  (CallFunction|ModifyMesh))

(event Collision|EventActorBeginOverlap
  (params (OtherActor :type Actor%20Object%20Reference))
  ;[0.15 0.15 0.15 0.5] Trigger and Collision
)

(event EventTick
  (params (DeltaSeconds :type Float%20%28single-precision%29))
  (CallFunction|MoveMesh DeltaSeconds)
  (Utilities|FlowControl|Delay 1.0)
  (CallFunction|RandomizedLight))

(event Collision|EventHit
  (params (MyComp :type Primitive%20Component%20Object%20Reference) (Other :type Actor%20Object%20Reference) (OtherComp :type Primitive%20Component%20Object%20Reference) (bSelfMoved :type Boolean) (HitLocation :type Vector :default "0, 0, 0") (HitNormal :type Vector :default "0, 0, 0") (NormalImpulse :type Vector :default "0, 0, 0") (Hit :type Hit%20Result%20Structure%20%28by%20ref%29))
  ;[0.15 0.15 0.15 0.5] Trigger and Collision
)

(fn ConstructionScript)

(fn ModifyMesh
  (bind _mymesh (Variables|Default|GetMyMesh))
  (Transformation|AddWorldOffset _mymesh "0.000000,0.000000,10.000000" false false)
  (Transformation|AddWorldRotation _mymesh "0.000000,45.000000,0.000000" false false)
  (Transformation|SetWorldScale3D _mymesh "2.000000,2.000000,1.000000")
  (Components|StaticMesh|SetStaticMesh _mymesh "/Engine/VREditor/BasicMeshes/SM_Pyramid_01.SM_Pyramid_01"))

(fn RandomizedLight
  (bind _pointlight (Variables|Default|GetPointLight))
  (Rendering|Components|Light|SetIntensity _pointlight (Math|Random|RandomFloatinRange (Variables|Light|GetLightIntensity_Min) (Variables|Light|GetLightIntensity_Max)))
  (Rendering|Components|Light|SetLightColor _pointlight (.OutItem (Utilities|Array|Random (Utilities|Array|MakeArray "(R=0.627541,G=1.000000,B=0.000000,A=1.000000)" "(R=1.000000,G=0.024018,B=0.000000,A=1.000000)" "(R=0.000000,G=0.991164,B=1.000000,A=1.000000)" "(R=0.001251,G=0.510417,B=0.123269,A=1.000000)"))) true))

(fn MoveMesh
  (params (DeltaSeconds :type Float%20%28single-precision%29))
  (Transformation|AddWorldOffset (Variables|Default|GetDefaultSceneRoot) (* "0.000000,0.000000,20.000000" DeltaSeconds) false false))